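; Snow plane actor that prepares a surface material to receive a footstep canvas texture.
; The construction script creates a dynamic instance of the snow material and applies it to the static mesh.
; On BeginPlay it creates a square canvas render target at a configurable size, binds it to the material's footstep parameter and updates it.
; No footstep drawing happens in this Blueprint.
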(event `self.ReceiveBeginPlay`
  (bind _canvas_size (`self.Canvas size`))
  (bind _returnvalue (`CanvasRenderTarget2D.CreateCanvasRenderTarget2D` "/Script/Engine.CanvasRenderTarget2D" _canvas_size _canvas_size))
  (bind _output_get (set `self.Snow Canvas` _returnvalue))
  (`MaterialInstanceDynamic.SetTextureParameterValue` (`self.dyn Mat`) "footstepCanvas" _output_get)
  (`CanvasRenderTarget2D.UpdateResource` _output_get))

(fn `UserConstructionScript`
  (bind _returnvalue (`KismetMaterialLibrary.CreateDynamicMaterialInstance` (`self.Snow Material`)))
  (bind _output_get (set `self.dyn Mat` _returnvalue))
  (`PrimitiveComponent.SetMaterial` (`self.StaticMeshComponent`) 0 _output_get))