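; Sphere actor that imprints its shape as a trail onto the snow plane's canvas as it moves.
; Creates a render target for DepthCaptureCam, which it keeps 90 units below the mesh, looking up at it.
; When pelvisSocket moves beyond a small tolerance, a downward trace looks for a Snow_Plane_Blueprint.
; On a hit, it additively draws the capture into SnowCanvas at the collision UV, scaled by FootSize with StepStrength as alpha.
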(event `self.ReceiveBeginPlay`
  (bind _captureres (`self.CaptureRes`))
  (bind _returnvalue (`KismetRenderingLibrary.CreateRenderTarget2D` _captureres _captureres))
  (bind _output_get (set `self.DepthCaptureTarget` _returnvalue))
  (set `SceneCaptureComponent2D.TextureTarget` _output_get (`SceneCapture2D.CaptureComponent2D` (`self.DepthCaptureCam`))))

(event `self.ReceiveTick`
  (params (DeltaSeconds :type "Float (single-precision)"))
  (bind _staticmeshcomponent (`self.StaticMeshComponent`))
  (bind _returnvalue (`SceneComponent.K2_GetComponentLocation` (`self.StaticMeshComponent`)))
  (bind _returnvalue_2 (`SceneComponent.GetSocketLocation` _staticmeshcomponent "pelvisSocket"))
  (bind _returnvalue_3 (- _returnvalue (0.0 0.0 90.0)))
  (`self.K2_SetActorLocationAndRotation` (`self.DepthCaptureCam`) _returnvalue_3 (`KismetMathLibrary.FindLookAtRotation` _returnvalue_3 _returnvalue) false true)
  (if (!= (`self.LastPosition`) _returnvalue_2 :`ErrorTolerance` 10.0)
    (set `self.Rotate foot` (`SceneComponent.GetSocketRotation` _staticmeshcomponent "pelvisSocket"))
    (set `self.LastPosition` _returnvalue_2)
    (bind (_outhit _returnvalue_4) (`KismetSystemLibrary.LineTraceSingle` :`Start` _returnvalue_2 :`End` (+ _returnvalue_2 (`KismetMathLibrary.MakeVector` 0.0 0.0 (* -1 (`self.Raytrace distance`)))) :`TraceChannel` "TraceTypeQuery1" :`bTraceComplex` true :`DrawDebugType` (`self.Ray debug`) :`DrawTime` 0.05))
    (if _returnvalue_4
      (bind _assnow_plane_blueprint (cast `/Game/Blueprints/Snow_Plane_Blueprint` (`.HitActor` (`GameplayStatics.BreakHitResult` _outhit))))
      (bind (_canvas _size _context) (`KismetRenderingLibrary.BeginDrawCanvasToRenderTarget` (`/Game/Blueprints/Snow_Plane_Blueprint.Snow Canvas` _assnow_plane_blueprint)))
      (bind (_screen_position _screen_size) (`/Engine/ArtTools/RenderToTexture/Macros/RenderToTextureFunctionLibrary.Set Canvas Material Scale and Position` _size (`GameplayStatics.FindCollisionUV` _outhit) (`self.Foot size`)))
      (`Canvas.K2_DrawTexture` _canvas (`self.DepthCaptureTarget`) _screen_position _screen_size (0.0 0.0) (1.0 1.0) (`KismetMathLibrary.MakeColor` 0.0 0.0 -1.0 (`self.Step strength`)) "BLEND_Additive" 90.0 (0.5 0.5))
      (`KismetRenderingLibrary.EndDrawCanvasToRenderTarget` _context))))

(fn `UserConstructionScript`)